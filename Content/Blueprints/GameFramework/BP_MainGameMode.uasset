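; BP_MainGameMode is the game mode Blueprint that extends parent logic for game start and idle NPC returns.
; BeginPlay applies saved user settings.
; StartGame creates the player controller's HUD with a level-based time limit, unpauses the game and starts a looping computer hum.
; ReturnIdleNPC teleports the character to the NPC spawn point's transform before handing off to the parent.
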(event `self.ReceiveBeginPlay`
  (`parent.ReceiveBeginPlay`)
  (bind _returnvalue (`GameUserSettings.GetGameUserSettings`))
  (`GameUserSettings.ApplySettings` _returnvalue true))

(event `self.StartGame`
  (params (DifficultyLevel :type Integer))
  (`parent.StartGame` DifficultyLevel)
  (`|ExecutionSequence`
    (:`then_0`
      (bind _asbp_player_controller (cast `/Game/Blueprints/GameFramework/BP_PlayerController` (`GameplayStatics.GetPlayerController` 0)))
      (bind _returnvalue (`|CreateWidget` "/Game/Blueprints/UI/WBP_HUD.WBP_HUD_C" _asbp_player_controller))
      (`/Game/Blueprints/UI/WBP_HUD.SetTimeLimit` _returnvalue (select `int` (`self.Level`) :`0` 0.0 :`1` 15.0 :`2` 15.0 :`3` 15.0))
      (bind _output_get (set `/Game/Blueprints/GameFramework/BP_PlayerController.HUD` _returnvalue _asbp_player_controller))
      (`UserWidget.AddToViewport` _output_get 0)
      (`GameplayStatics.SetGamePaused` false))
    (:`then_1`
      (bind _returnvalue_2 (`GameplayStatics.SpawnSoundAtLocation` "/Game/Sound/Computer_Hum_Loop_Cue.Computer_Hum_Loop_Cue" (0.0 0.0 0.0) (struct) 1.0 1.0 0.0 null null))
      (set `self.HumLoop` _returnvalue_2))))

(event `self.ReturnIdleNPC`
  (params (Character :type "Character Object Reference") (bIsArrest :type Boolean))
  (`self.K2_SetActorTransform` Character (`self.GetTransform` (`|ConvertAsset` (`self.NPCSpawnPoint`))) false false)
  (`parent.ReturnIdleNPC` Character bIsArrest))

(fn `UserConstructionScript`)