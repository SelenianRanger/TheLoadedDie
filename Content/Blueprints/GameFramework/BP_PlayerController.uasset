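; Player controller that opens the game on a paused main menu and provides a pause menu.
; Shortly after BeginPlay it pauses and shows WBP_MainMenu with UI-only input; Escape does the same with WBP_PauseMenu.
; The I, P and O keys halve, double and reset global time dilation.
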(event `self.ReceiveBeginPlay`
  (`KismetSystemLibrary.Delay` 0.1)
  (`GameplayStatics.SetGamePaused` true)
  (bind _returnvalue (`|CreateWidget` "/Game/Blueprints/UI/WBP_MainMenu.WBP_MainMenu_C" self))
  (`UserWidget.AddToViewport` _returnvalue 0)
  (`WidgetBlueprintLibrary.SetInputMode_UIOnlyEx` self _returnvalue))

(event `Key|Escape`
  (params (Key :type "Key Structure"))
  (:`Pressed`
    (bind _returnvalue (`|CreateWidget` "/Game/Blueprints/UI/WBP_PauseMenu.WBP_PauseMenu_C" self))
    (`UserWidget.AddToViewport` _returnvalue 0)
    (`WidgetBlueprintLibrary.SetInputMode_UIOnlyEx` self _returnvalue)
    (`GameplayStatics.SetGamePaused` true)))

(event `Key|I`
  (params (Key :type "Key Structure"))
  (:`Pressed`
    (`GameplayStatics.SetGlobalTimeDilation` (/ (`GameplayStatics.GetGlobalTimeDilation`) 2.0))))

(event `Key|P`
  (params (Key :type "Key Structure"))
  (:`Pressed`
    (`GameplayStatics.SetGlobalTimeDilation` (* (`GameplayStatics.GetGlobalTimeDilation`) 2.0))))

(event `Key|O`
  (params (Key :type "Key Structure"))
  (:`Pressed`
    (`GameplayStatics.SetGlobalTimeDilation` 1.0)))

(fn `UserConstructionScript`)