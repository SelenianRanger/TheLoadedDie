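; BP_GameTable is a dice table that runs the NPC cycle of dealer, player and security guard.
; It borrows players from MainGameMode, walks them via AIMoveTo, loops matches on slot overlap, and returns them when they leave or get arrested.
; Dealer breaks let saboteurs load the dealer's dice, with polling timers gating movement.
; Thrown dice are visual, and players flagged both cheater and stupid can show rigged colors.
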(event `self.ReceiveBeginPlay`
  ;[1 1 1] Begin Play
  (`|ExecutionSequence`
    (:`then_0`
      ;;[1 1 1] Spawn security NPC
      (bind _returnvalue (`|SpawnActorFromClass` "/Game/Blueprints/Characters/NPC/BP_NPC_Dealer.BP_NPC_Dealer_C" (`SceneComponent.K2_GetComponentToWorld` (`self.DealerSpawnBillboard`)) "Undefined" "OverrideRootScale" null null))
      (set `self.SecurityNPC` _returnvalue))
    (:`then_1`
      ;;[1 1 1] Spawn Dealer
      (bind _returnvalue_2 (`|SpawnActorFromClass` "/Game/Blueprints/Characters/NPC/BP_NPC_Dealer.BP_NPC_Dealer_C" (`SceneComponent.K2_GetComponentToWorld` (`self.DealerSpawnBillboard`)) "Undefined" "OverrideRootScale" null null))
      (set `self.DealerNPC` _returnvalue_2)
      (`KismetSystemLibrary.Delay` (`KismetMathLibrary.RandomFloatInRange` 1.0 6.0))
      (`self.ReturnDealerToTable`))
    (:`then_2`
      ;;[1 1 1] Player Request loop
      (`KismetSystemLibrary.K2_SetTimerDelegate` (delegate `CheckForPlayer`) 10.0 true (`KismetMathLibrary.RandomFloatInRange` 2.0 5.0)))))

(event `CheckForPlayer`
  ;[1 1 1] Begin Play
  ;;[1 1 1] Player Request loop
  (`/Engine/EditorBlueprintResources/StandardMacros.IsValid` (`self.PlayerNPC`)
    (:`Is Not Valid`
      (`self.RequestNewPlayer`))))

(event `PlayLoop`
  ;[1 1 1] Play Loop
  ;;[1 1 1] Pre Match Delay
  (`KismetSystemLibrary.Delay` (`KismetMathLibrary.RandomFloatInRange` 0.5 2.0))
  ;;[1 1 1] Throw the visual dice
  (bind _asbp_npc_player (cast `/Game/Blueprints/Characters/NPC/BP_NPC_Player` (`self.PlayerNPC`)))
  (`self.ThrowDice` (and (`NPC_PlayerCharacter.bIsCheater` _asbp_npc_player) (`NPC_PlayerCharacter.bIsStupid` _asbp_npc_player)))
  (`KismetSystemLibrary.Delay` 2.0)
  (`self.PlayMatch`)
  ;;[1 1 1] Check if NPC wants to leave
  (bind _asbp_npc_player_2 (cast `/Game/Blueprints/Characters/NPC/BP_NPC_Player` (`self.PlayerNPC`)))
  (if (not (`NPC_PlayerCharacter.WantsToLeave` _asbp_npc_player_2))
    ;;[1 1 1] Post Match Delay
    (`KismetSystemLibrary.Delay` (`KismetMathLibrary.RandomFloatInRange` 5.0 8.0))
    (`self.PlayLoop`)
    (else
      ;;[1 1 1] Have player leave
      (`KismetSystemLibrary.Delay` (`KismetMathLibrary.RandomFloatInRange` 2.0 4.0))
      (`self.OrderPlayerToLeave` false))))

(event `self.DealerSlotCollision.OnComponentBeginOverlap`
  (params (OverlappedComponent :type "PrimitiveComponent Object Reference") (OtherActor :type "Actor Object Reference") (OtherComp :type "PrimitiveComponent Object Reference") (OtherBodyIndex :type Integer) (bFromSweep :type Boolean) (SweepResult :type "HitResult Structure (by ref)"))
  ;[0.5625 0.5625 0.5625] Collision checks
  (`|ExecutionSequence`
    (:`then_0`
      ;;[1 1 1] Check if dealer is coming back from break
      (if (== OtherActor (`self.DealerNPC`))
        (set `self.bIsDealerOnBreak` false)
        ;;[1 1 1] Snap dealer into place
        (`NavMovementComponent.StopActiveMovement` (`Character.CharacterMovement` (`self.DealerNPC`)))
        (`self.K2_SetActorTransform` (`self.DealerNPC`) (`SceneComponent.K2_GetComponentToWorld` (`self.DealerSlotCollision`)) false false)))
    (:`then_1`
      ;;[1 1 1] Check if player has come to sabotage
      (if (== OtherActor (`self.PlayerNPC`))
        (set `self.bIsRigged` true)
        ;;[1 1 1] Rig dealer dice
        (`DiceD6.SetDiceType` (`self.DiceD6`) "EDLT_LoadedLowRoller")))))

(event `self.ThrowDice`
  (params (bIsDiceRigged :type Boolean))
  (bind _returnvalue (not bIsDiceRigged))
  (bind _returnvalue_2 (and (`KismetMathLibrary.RandomBool`) bIsDiceRigged))
  ;[0.5625 0.5625 0.5625] Throw Dice (Visual)
  (`|ExecutionSequence`
    (:`then_0`
      ;;[1 1 1] Spawn Player Die
      (bind _returnvalue_3 (`|SpawnActorFromClass` "/Game/Blueprints/Actors/BP_Dice.BP_Dice_C" (`SceneComponent.K2_GetComponentToWorld` (`self.PlayerDiceSpawnBillboard`)) "Undefined" "OverrideRootScale" null null))
      (if _returnvalue
        (`Dice.SetColor` _returnvalue_3 "Player")
        (elif _returnvalue_2
          (`Dice.SetColor` _returnvalue_3 "Rigged")
          (else
            (`Dice.SetColor` _returnvalue_3 "Player"))))
      (`KismetSystemLibrary.Delay` (`self.DiceThrowDelayShort`))
      (bind _returnvalue_4 (`|SpawnActorFromClass` "/Game/Blueprints/Actors/BP_Dice.BP_Dice_C" (`SceneComponent.K2_GetComponentToWorld` (`self.PlayerDiceSpawnBillboard`)) "Undefined" "OverrideRootScale" null null))
      (if _returnvalue
        (`Dice.SetColor` _returnvalue_4 "Player")
        (elif (not _returnvalue_2)
          (`Dice.SetColor` _returnvalue_4 "Rigged")
          (else
            (`Dice.SetColor` _returnvalue_4 "Player")))))
    (:`then_1`
      (`KismetSystemLibrary.Delay` (`self.DiceThrowDelayLong`))
      ;;[1 1 1] Spawn Dealer Die
      (bind _returnvalue_5 (`|SpawnActorFromClass` "/Game/Blueprints/Actors/BP_Dice.BP_Dice_C" (`SceneComponent.K2_GetComponentToWorld` (`self.DealerDiceSpawnBillboard`)) "Undefined" "OverrideRootScale" null null))
      (`Dice.SetColor` _returnvalue_5 "Dealer")
      (`KismetSystemLibrary.Delay` (`self.DiceThrowDelayShort`))
      (bind _returnvalue_6 (`|SpawnActorFromClass` "/Game/Blueprints/Actors/BP_Dice.BP_Dice_C" (`SceneComponent.K2_GetComponentToWorld` (`self.DealerDiceSpawnBillboard`)) "Undefined" "OverrideRootScale" null null))
      (`Dice.SetColor` _returnvalue_6 "Dealer"))))

(event `self.PlayerSlotCollision.OnComponentBeginOverlap`
  (params (OverlappedComponent :type "PrimitiveComponent Object Reference") (OtherActor :type "Actor Object Reference") (OtherComp :type "PrimitiveComponent Object Reference") (OtherBodyIndex :type Integer) (bFromSweep :type Boolean) (SweepResult :type "HitResult Structure (by ref)"))
  ;[0.5625 0.5625 0.5625] Collision checks
  ;;[1 1 1] Check if player has come to play
  (if (== OtherActor (`self.PlayerNPC`))
    (set `self.bIsGameInProgress` true)
    ;;[1 1 1] Snap player into place
    (`NavMovementComponent.StopActiveMovement` (`Character.CharacterMovement` (`self.PlayerNPC`)))
    (`self.K2_SetActorTransform` (`self.PlayerNPC`) (`SceneComponent.K2_GetComponentToWorld` (`self.PlayerSlotCollision`)) false false)
    ;;[1 1 1] start play loop
    (`self.PlayLoop`)))

(event `self.RequestNewPlayer`
  ;[0.5625 0.5625 0.5625] NPC Tasks
  ;;[0.5625 0.5625 0.5625] Request New Player
  ;;;[1 1 1] Request new player
  (bind _asmain_game_mode (cast `MainGameMode` (`GameplayStatics.GetGameMode`)))
  (bind _returnvalue (`MainGameMode.AskForNPCPlayer` _asmain_game_mode))
  (`/Engine/EditorBlueprintResources/StandardMacros.IsValid` _returnvalue
    (:`Is Valid`
      (bind _output_get (set `self.PlayerNPC` _returnvalue))
      (`self.K2_SetActorLocation` _output_get (`SceneComponent.K2_GetComponentLocation` (`self.PlayerSpawnBillboard`)) false false)
      (`|ExecutionSequence`
        (:`then_0`
          ;;;[1 1 1] Saboteur Loop
          (bind _asbp_npc_player (cast `/Game/Blueprints/Characters/NPC/BP_NPC_Player` (`self.PlayerNPC`)))
          (if (`NPC_PlayerCharacter.bIsSaboteur` _asbp_npc_player)
            (bind _returnvalue_2 (`KismetSystemLibrary.K2_SetTimerDelegate` (delegate `TrySabotage`) 0.1 true))
            (set `self.SaboteurTimer` _returnvalue_2)))
        (:`then_1`
          ;;;[1 1 1] Delay before moving player to slot
          (bind _asbp_npc_player_2 (cast `/Game/Blueprints/Characters/NPC/BP_NPC_Player` (`self.PlayerNPC`)))
          (`KismetSystemLibrary.Delay` (select `bool` (`NPC_PlayerCharacter.bIsSaboteur` _asbp_npc_player_2) :`false` (`KismetMathLibrary.RandomFloatInRange` 1.0 8.0) :`true` (`KismetMathLibrary.RandomFloatInRange` 5.0 10.0)))
          (`KismetSystemLibrary.K2_ClearAndInvalidateTimerHandle` (`self.SaboteurTimer`))
          ;;;[1 1 1] Player move to slot loop
          (bind _returnvalue_3 (`KismetSystemLibrary.K2_SetTimerDelegate` (delegate `TryMoveToSlot`) 0.1 true))
          (set `self.PlayerSlotCheckTimer` _returnvalue_3))))))

(event `self.AskDealerToTakeBreak`
  ;[0.5625 0.5625 0.5625] NPC Tasks
  ;;[0.5625 0.5625 0.5625] Dealer
  ;;;[0.5625 0.5625 0.5625] Send Dealer On Break
  (if (> (`KismetMathLibrary.RandomFloatInRange` 0.0 1.0) 0.2)
    (set `self.bIsDealerOnBreak` true)
    ;;;;[1 1 1] Move Dealer to Break Spot
    (`|AIMoveTo` self (`self.DealerNPC`) (`SceneComponent.K2_GetComponentLocation` (`self.DealerSpawnBillboard`)) null
      (:`OnSuccess`
        (`KismetSystemLibrary.K2_SetTimerDelegate` (delegate `DealerReturnLoop`) (`KismetMathLibrary.RandomFloatInRange` 10.0 15.0))))))

(event `TrySabotage`
  ;[0.5625 0.5625 0.5625] NPC Tasks
  ;;[0.5625 0.5625 0.5625] Request New Player
  ;;;[1 1 1] Saboteur Loop
  (`self.MovePlayerToSabotage`))

(event `DealerReturnLoop`
  ;[0.5625 0.5625 0.5625] NPC Tasks
  ;;[0.5625 0.5625 0.5625] Dealer
  ;;;[0.5625 0.5625 0.5625] Send Dealer On Break
  (bind _returnvalue (`KismetSystemLibrary.K2_SetTimerDelegate` (delegate `ReturnDealerToTable`) 0.2 true))
  (set `self.DealerReturnTimer` _returnvalue))

(event `ReturnDealerToTable`
  ;[0.5625 0.5625 0.5625] NPC Tasks
  ;;[0.5625 0.5625 0.5625] Dealer
  (if (not (`self.bIsBeingSabotaged`))
    (`KismetSystemLibrary.K2_ClearAndInvalidateTimerHandle` (`self.DealerReturnTimer`))
    ;;;[1 1 1] Move Dealer to Table Slot
    (`|AIMoveTo` self (`self.DealerNPC`) (`SceneComponent.K2_GetComponentLocation` (`self.DealerSlotCollision`)) null)))

(event `TryMoveToSlot`
  ;[0.5625 0.5625 0.5625] NPC Tasks
  ;;[0.5625 0.5625 0.5625] Request New Player
  ;;;[1 1 1] Player move to slot loop
  (`self.MovePlayerToSlot`))

(event `self.OrderPlayerToLeave`
  (params (bIsArrest :type Boolean))
  ;[0.5625 0.5625 0.5625] NPC Tasks
  ;;[0.5625 0.5625 0.5625] Player
  (`/Engine/EditorBlueprintResources/StandardMacros.IsValid` (`self.PlayerNPC`)
    (:`Is Valid`
      (set `self.bIsGameInProgress` false)
      (set `self.bIsRigged` false)
      (`DiceD6.SetDiceType` (`self.DiceD6`) "ELDT_NotLoaded")
      ;;;[1 1 1] Move player out of scene
      (`|AIMoveTo` self (`self.PlayerNPC`) (`SceneComponent.K2_GetComponentLocation` (`self.PlayerSpawnBillboard`)) null
        (:`OnSuccess`
          ;;;[1 1 1] Return NPC ownership to gamemode to handle
          (bind _asmain_game_mode (cast `MainGameMode` (`GameplayStatics.GetGameMode`)))
          (`MainGameMode.ReturnIdleNPC` _asmain_game_mode (`self.PlayerNPC`) bIsArrest)
          (set `self.PlayerNPC` null)
          (`self.AskDealerToTakeBreak`))))))

(event `self.MovePlayerToSlot`
  ;[0.5625 0.5625 0.5625] NPC Tasks
  ;;[0.5625 0.5625 0.5625] Player
  (`/Engine/EditorBlueprintResources/StandardMacros.IsValid` (`self.PlayerNPC`)
    (:`Is Valid`
      (if (not (`self.bIsDealerOnBreak`))
        (`KismetSystemLibrary.K2_ClearAndInvalidateTimerHandle` (`self.PlayerSlotCheckTimer`))
        ;;;[1 1 1] Move player to table slot
        (`|AIMoveTo` self (`self.PlayerNPC`) (`SceneComponent.K2_GetComponentLocation` (`self.PlayerSlotCollision`)) null)))))

(event `self.ArrestPlayer`
  (bind _securitynpc (`self.SecurityNPC`))
  (bind _securitynpc_2 (`self.SecurityNPC`))
  (bind _securitynpc_3 (`self.SecurityNPC`))
  ;[0.5625 0.5625 0.5625] NPC Tasks
  ;;[0.5625 0.5625 0.5625] Player
  (`/Engine/EditorBlueprintResources/StandardMacros.IsValid` (`self.PlayerNPC`)
    (:`Is Valid`
      (`NavMovementComponent.StopActiveMovement` (`Character.CharacterMovement` (`self.PlayerNPC`)))
      ;;;[1 1 1] Move security to player
      (`|AIMoveTo` _securitynpc_2 _securitynpc_2 (`self.K2_GetActorLocation` (`self.PlayerNPC`)) null 150.0
        (:`OnSuccess`
          (`KismetSystemLibrary.Delay` 2.0)
          ;;;[1 1 1] Escort player out of scene
          (`|AIMoveTo` _securitynpc_3 _securitynpc_3 (`SceneComponent.K2_GetComponentLocation` (`self.PlayerSpawnBillboard`)) null 150.0
            (:`then`
              (`KismetSystemLibrary.Delay` 0.5)
              (`self.OrderPlayerToLeave` true))
            (:`OnSuccess`
              (`|AIMoveTo` _securitynpc _securitynpc (`SceneComponent.K2_GetComponentLocation` (`self.DealerSpawnBillboard`)) null 150.0))))))))

(event `self.MovePlayerToSabotage`
  ;[0.5625 0.5625 0.5625] NPC Tasks
  ;;[0.5625 0.5625 0.5625] Player
  (`/Engine/EditorBlueprintResources/StandardMacros.IsValid` (`self.PlayerNPC`)
    (:`Is Valid`
      (if (`self.bIsDealerOnBreak`)
        (`KismetSystemLibrary.K2_ClearAndInvalidateTimerHandle` (`self.SaboteurTimer`))
        (set `self.bIsBeingSabotaged` true)
        ;;;[1 1 1] Move player to sabotage slot
        (`|AIMoveTo` self (`self.PlayerNPC`) (`SceneComponent.K2_GetComponentLocation` (`self.DealerSlotCollision`)) null
          (:`OnSuccess`
            (`KismetSystemLibrary.Delay` 2.0)
            ;;;[1 1 1] Move player to spawn position
            (`|AIMoveTo` self (`self.PlayerNPC`) (`SceneComponent.K2_GetComponentLocation` (`self.PlayerSpawnBillboard`)) null
              (:`OnSuccess`
                (set `self.bIsBeingSabotaged` false)))))))))

(fn `UserConstructionScript`)