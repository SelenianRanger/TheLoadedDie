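; BP_SwayingLight is a light actor that sways by rotating itself in roll and pitch.
; On BeginPlay it plays two timelines, each given a random value up to RollOffset or PitchOffset, which varies the motion between instances.
; The roll timeline's update sets actor rotation from both timeline values, scaled by RollAmount and PitchAmount.
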(event `self.ReceiveBeginPlay`
  (`|ExecutionSequence`
    (:`then_0`
      (bind (_direction _value) (`Timeline|Timeline_0` :`NewTime` (`KismetMathLibrary.RandomFloatInRange` 0.0 (`self.RollOffset`)))
        (:`Update`
          (`self.K2_SetActorRotation` (`KismetMathLibrary.MakeRotator` (* _value (`self.RollAmount`)) (* (stale _value_2) (`self.PitchAmount`)))))))
    (:`then_1`
      (bind (_direction_2 _value_2) (`Timeline|Timeline_1` :`NewTime` (`KismetMathLibrary.RandomFloatInRange` 0.0 (`self.PitchOffset`)))))))

(fn `UserConstructionScript`)