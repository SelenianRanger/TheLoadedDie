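; Clickable security-style monitor that shows camera channels and dice match results, with power and next-channel buttons.
; It binds to channel changes and starts on a random channel, showing a timed noise screen and re-checking power before applying the new material and name.
; While powered, match results briefly show both sides' rolls, a win/loss light and profit signed from the house's perspective, negative when the player wins.
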(event `SetNewChannel` :!signature `self.OnChannelChanged`
  (params (NewCameraChannel :type "CameraChannel Structure"))
  (bind (_cctv _materialinstance _name) (break `CameraChannel` NewCameraChannel))
  ;[1 1 1] Channel Changed
  (if (`self.bTurnedOn`)
    (`PrimitiveComponent.SetMaterialByName` (`self.Monitor`) "Power Button" "/Game/Materials/Monitor/MI_Emissive_Green.MI_Emissive_Green")
    (`PrimitiveComponent.SetMaterial` (`self.Screen`) 0 "/Game/Materials/Monitor/Screens/MI_Screen_Noise.MI_Screen_Noise")
    (`TextRenderComponent.K2_SetText` (`self.CameraText`) "")
    (`KismetSystemLibrary.Delay` (`self.TransitionDuration`))
    (if (`self.bTurnedOn`)
      (`PrimitiveComponent.SetMaterial` (`self.Screen`) 0 _materialinstance :!label _label)
      (`TextRenderComponent.K2_SetText` (`self.CameraText`) _name)
      (`SceneComponent.SetVisibility` (`self.CameraText`) true false))
    (else
      (`PrimitiveComponent.SetMaterialByName` (`self.Monitor`) "Power Button" "/Game/Materials/Monitor/MI_Emissive_Red.MI_Emissive_Red")
      (goto _label))))

(event `self.ReceiveBeginPlay`
  (`|ExecutionSequence`
    (:`then_0`
      ;[1 1 1] Channel Changed
      (add `self.OnChannelChanged` (delegate `SetNewChannel`)))
    (:`then_1`
      (`self.GoRandomChannel`))))

(event `SetDisplayVisibility`
  (params (`Turned On` :type Boolean))
  ;[1 1 1] Set Display Visibility
  (`SceneComponent.SetVisibility` (`self.Dice Texts`) `Turned On` true)
  (`SceneComponent.SetVisibility` (`self.ProfitText`) `Turned On` true)
  (`SceneComponent.SetVisibility` (`self.CameraText`) (or `Turned On` (`self.bTurnedOn`)) true)
  (if (not `Turned On`)
    (`PrimitiveComponent.SetMaterialByName` (`self.Side_Displays`) "Light Left" "/Game/Materials/Monitor/MI_Monitor_Light_Off.MI_Monitor_Light_Off")
    (`PrimitiveComponent.SetMaterialByName` (`self.Side_Displays`) "Light Right" "/Game/Materials/Monitor/MI_Monitor_Light_Off.MI_Monitor_Light_Off")))

(event `self.UpdateMatchResultDisplay`
  (params (MatchResult :type "MatchResult Structure"))
  (bind (_playerdiceoneroll _playerdicetworoll _dealerdiceoneroll _dealerdicetworoll _playerwon _bet) (break `MatchResult` MatchResult))
  ;[0.4635 0.4635 0.4635] Update Match Result Display
  (if (`self.bTurnedOn`)
    (`self.SetDisplayVisibility` false)
    (`|ExecutionSequence`
      (:`then_0`
        ;;[1 1 1] set visibility
        (`self.SetDisplayVisibility` true)
        (`KismetSystemLibrary.Delay` (`self.MatchDisplayTimeout`))
        (`self.SetDisplayVisibility` false))
      (:`then_1`
        ;;[1 1 1] Lights
        (if _playerwon
          (`PrimitiveComponent.SetMaterialByName` (`self.Side_Displays`) "Light Left" "/Game/Materials/Monitor/MI_Emissive_Green.MI_Emissive_Green")
          (else
            (`PrimitiveComponent.SetMaterialByName` (`self.Side_Displays`) "Light Right" "/Game/Materials/Monitor/MI_Emissive_Red.MI_Emissive_Red"))))
      (:`then_2`
        ;;[1 1 1] Profit Text
        (`TextRenderComponent.K2_SetText` (`self.ProfitText`) (`|FormatText` "{sign}${amount}" (select `bool` _playerwon :`false` "+" :`true` "-" :!type "Text") _bet))
        ;;[1 1 1] Dice Rolls
        (`TextRenderComponent.K2_SetText` (`self.PlayerRoll1Text`) (`KismetTextLibrary.Conv_IntToText` _playerdiceoneroll))
        (`TextRenderComponent.K2_SetText` (`self.PlayerRoll2Text`) (`KismetTextLibrary.Conv_IntToText` _playerdicetworoll))
        (`TextRenderComponent.K2_SetText` (`self.DealerRoll1Text`) (`KismetTextLibrary.Conv_IntToText` _dealerdiceoneroll))
        (`TextRenderComponent.K2_SetText` (`self.DealerRoll2Text`) (`KismetTextLibrary.Conv_IntToText` _dealerdicetworoll))))))

(event `self.NextCollision.OnClicked`
  (params (TouchedComponent :type "PrimitiveComponent Object Reference") (ButtonPressed :type "Key Structure"))
  ;[1 1 1] Next Channel Button
  (`GameplayStatics.PlaySoundAtLocation` "/Game/Sound/Button02_Cue.Button02_Cue" (`self.K2_GetActorLocation`) (struct) 1.0 1.0 0.0 null null null null)
  (`self.GoNextChannel`)
  (`self.SetDisplayVisibility` false))

(event `self.PowerCollision.OnClicked`
  (params (TouchedComponent :type "PrimitiveComponent Object Reference") (ButtonPressed :type "Key Structure"))
  ;[1 1 1] Power Button
  (`GameplayStatics.PlaySoundAtLocation` "/Game/Sound/Button01_Cue.Button01_Cue" (`self.K2_GetActorLocation`) (struct) 1.0 1.0 0.0 null null null null)
  (`self.TogglePower`)
  (if (not (`self.bTurnedOn`))
    (`self.SetDisplayVisibility` false)))

(fn `UserConstructionScript`)