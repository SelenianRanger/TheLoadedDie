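; BP_Dice is a physics-driven die actor that gets thrown as soon as it spawns.
; On BeginPlay it sets its lifespan, applies a random-axis, random-magnitude torque as an acceleration change, and adds an impulse along the actor's forward vector scaled by ImpulseStrength.
; The spawn rotation therefore sets the throw direction, while the random torque varies the tumble.
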(event `self.ReceiveBeginPlay`
  (`self.SetLifeSpan` (`self.LifeSpan`))
  (`PrimitiveComponent.AddTorqueInDegrees` (`self.Mesh`) (* (`KismetMathLibrary.RandomFloatInRange` 20.0 50.0) 1000.0 (`KismetMathLibrary.RandomUnitVector`)) "None" true)
  (`PrimitiveComponent.AddImpulse` (`self.Mesh`) (* (`self.ImpulseStrength`) 1000.0 (`self.GetActorForwardVector`)) "None" false))

(fn `UserConstructionScript`)