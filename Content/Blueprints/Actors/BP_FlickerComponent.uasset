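; Actor component that makes its owner flicker by toggling its hidden-in-game state in random bursts, with occasional jump scares.
; Tick uses latent Delays for a random first-run offset and the gap between bursts, then picks a blink count.
; Flicker hides and reshows the owner, re-calling itself until the count runs out.
; Each blink has a small chance to briefly reveal the JumpScareActors, without holding up the flicker sequence.
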(event `self.ReceiveTick`
  (params (DeltaSeconds :type "Float (single-precision)"))
  (if (`self.bFirstTime`)
    (`KismetSystemLibrary.Delay` (`KismetMathLibrary.RandomFloatInRange` 0.0 30.0))
    (set `self.bFirstTime` false))
  (`KismetSystemLibrary.Delay` (`KismetMathLibrary.RandomFloatInRange` (`self.FlickerDelayMin`) (`self.FlickerDelayMax`)))
  (set `self.IterationsLeft` (`KismetMathLibrary.RandomIntegerInRange` (`self.FlickerCountMin`) (`self.FlickerCountMax`)))
  (`self.Flicker`))

(event `Flicker`
  (`Actor.SetActorHiddenInGame` (`self.GetOwner`) true)
  (`KismetSystemLibrary.Delay` (`self.FlickerPeriod`))
  (`Actor.SetActorHiddenInGame` (`self.GetOwner`) false)
  (`|ExecutionSequence`
    (:`then_0`
      (if (`KismetMathLibrary.RandomBoolWithWeight` 0.01)
        (if (`KismetArrayLibrary.Array_IsNotEmpty` (`self.JumpScareActors`))
          (for _array_element (`self.JumpScareActors`)
            (bind _output (`|ConvertAsset` _array_element))
            (`Actor.SetActorHiddenInGame` _output false)
            (`KismetSystemLibrary.Delay` (* (`self.FlickerPeriod`) 3.5))
            (`Actor.SetActorHiddenInGame` _output true)))))
    (:`then_1`
      (`KismetSystemLibrary.Delay` (`self.FlickerPeriod`))
      (bind _result (`/Engine/EditorBlueprintResources/StandardMacros.DecrementInt` (`self.IterationsLeft`))
        (:`  `
          (if (> _result 0)
            (`self.Flicker`)))))))